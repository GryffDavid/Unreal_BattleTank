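; Player-controllable tank Blueprint that wires its components together and maps input to aiming, driving and firing.
; BeginPlay registers the barrel and turret and initialises TankMovement with both tracks.
; Camera axes rotate an azimuth gimbal and spring arm, scaled by delta time.
; Driving supports direct per-track throttle or intent-based forward and rotate input through TankMovement, while the Fire action calls Fire.
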(event EventBeginPlay
  (Class|Tank|SetBarrelReference (Variables|Default|GetTankBarrel2))
  (Class|Tank|SetTurretReference (Variables|Default|GetTankTurret))
  (Class|TankMovementComponent|Initialise (Variables|Default|GetTankMovement) (Variables|Default|GetTrackL) (Variables|Default|GetTrackR)))

(event Collision|EventActorBeginOverlap
  (params (OtherActor :type Actor%20Object%20Reference)))

(event EventTick
  (params (DeltaSeconds :type Float%20%28single-precision%29)))

(event Input|ActionEvents|InputActionFire
  (params (Key :type Key%20Structure :default "None"))
  ;[1 1 1] Direct Movement Handling
  (:Pressed
    (Class|Tank|Fire)))

(event Input|AxisEvents|InputAxisAimAzimuth
  (params (AxisValue :type Float%20%28single-precision%29))
  ;[1 1 1] Handle Camera
  (Transformation|AddLocalRotation (Variables|Default|GetAzimuthGimbal) (Math|Rotator|MakeRotator 0.0 0.0 (* AxisValue (Utilities|Time|GetWorldDeltaSeconds) 1e+02)) false false))

(event Input|AxisEvents|InputAxisAimElevation
  (params (AxisValue :type Float%20%28single-precision%29))
  ;[1 1 1] Handle Camera
  (Transformation|AddLocalRotation (Variables|Default|GetCameraSpringArm) (Math|Rotator|MakeRotator 0.0 (* AxisValue (Utilities|Time|GetWorldDeltaSeconds) 1e+02) 0.0) false false))

(event Input|AxisEvents|InputAxisLeftTrackThrottle
  (params (AxisValue :type Float%20%28single-precision%29))
  ;[1 1 1] Direct Movement Handling
  (Class|TankTrack|SetThrottle (Variables|Default|GetTrackL) AxisValue))

(event Input|AxisEvents|InputAxisRightTrackThrottle
  (params (AxisValue :type Float%20%28single-precision%29))
  ;[1 1 1] Direct Movement Handling
  (Class|TankTrack|SetThrottle (Variables|Default|GetTrackR) AxisValue))

(event Input|AxisEvents|InputAxisMoveForward
  (params (AxisValue :type Float%20%28single-precision%29))
  (Class|TankMovementComponent|IntendMoveForward (Variables|Default|GetTankMovement) AxisValue))

(event Input|AxisEvents|InputAxisRotateTank
  (params (AxisValue :type Float%20%28single-precision%29))
  (Class|TankMovementComponent|IntendRotateClockwise (Variables|Default|GetTankMovement) AxisValue))

(fn ConstructionScript)